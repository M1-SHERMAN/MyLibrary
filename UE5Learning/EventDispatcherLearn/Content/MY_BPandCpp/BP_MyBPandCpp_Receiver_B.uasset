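; Blueprint actor that acts as a receiver in a Blueprint/C++ event dispatch example.
; It registers itself as a listener for the named event Bp_MyBPandCpp_DispatchEvent on BeginPlay and unregisters on EndPlay.
; When the event arrives, it casts the payload to MyData and prints its Param value on screen in blue.
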(event `self.ReceiveBeginPlay`
  (`parent.ReceiveBeginPlay`)
  (`MyEventManager.AddEventListener` "Bp_MyBPandCpp_DispatchEvent" self))

(event `self.OnReceiveEvent`
  (params (Data :type "Object Object Reference"))
  (`KismetSystemLibrary.PrintString` (`KismetStringLibrary.Concat_StrStr` "BP Receive Value: " (`KismetStringLibrary.Conv_IntToString` (`MyData.Param` (cast `MyData` Data :!pure true)))) true true (struct :`B` 1.0 :`A` 1.0) 5.0))

(event `self.ReceiveEndPlay`
  (params (EndPlayReason :type "EEndPlayReason Enum" :default "Destroyed"))
  (`MyEventManager.RemoveEventListener` "Bp_MyBPandCpp_DispatchEvent" self))

(fn `UserConstructionScript`
  (`parent.UserConstructionScript`))