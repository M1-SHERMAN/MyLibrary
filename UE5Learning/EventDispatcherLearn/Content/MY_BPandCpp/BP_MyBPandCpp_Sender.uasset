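; Sender Blueprint that periodically broadcasts a named event carrying a random integer payload, apparently as a test of Blueprint and C++ messaging.
; On BeginPlay it starts a looping timer bound to a custom event.
; Each firing creates a fresh MyData object, randomizes its Param, then passes it to DispatchEvent under a string event name, with no direct reference to any receiver.
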(event `self.ReceiveBeginPlay`
  (`parent.ReceiveBeginPlay`)
  (`KismetSystemLibrary.K2_SetTimerDelegate` (delegate `DoBPDispatchEvent`) 3.0 true))

(event `DoBPDispatchEvent`
  (`|ExecutionSequence`
    (:`then_0`
      (set `self.MyDataRef` (cast `MyData` (`MyEventManager.CreateNewData` "/Script/EventDispatcherLearn.MyData") :!pure true)))
    (:`then_1`
      (set `MyData.Param` (`KismetMathLibrary.RandomIntegerInRange` 0 100) (`self.MyDataRef`)))
    (:`then_2`
      (`MyEventManager.DispatchEvent` "Bp_MyBPandCpp_DispatchEvent" (`self.MyDataRef`)))))

(fn `UserConstructionScript`)